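; BP_Platform_JumpThru is a one-way platform that the player can jump up through and drop down through.
; A bottom trigger disables the Platform mesh collision while the player overlaps it and restores it when the overlap ends.
; A top trigger tracks whether the player stands on the platform, letting the IA_PlayerDown input disable collision to drop through.
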(event OnComponentBeginOverlap(BottomCollision)
  (params (OverlappedComponent :type Primitive%20Component%20Object%20Reference) (OtherActor :type Actor%20Object%20Reference) (OtherComp :type Primitive%20Component%20Object%20Reference) (OtherBodyIndex :type Integer) (bFromSweep :type Boolean) (SweepResult :type Hit%20Result%20Structure%20%28by%20ref%29))
  ;[1 0 1] Jump up THROUGH Platform
  (if (== OtherActor (Game|GetPlayerCharacter 0))
    (Collision|SetCollisionEnabled (Variables|Default|GetPlatform) "NoCollision")))

(event OnComponentEndOverlap(BottomCollision)
  (params (OverlappedComponent :type Primitive%20Component%20Object%20Reference) (OtherActor :type Actor%20Object%20Reference) (OtherComp :type Primitive%20Component%20Object%20Reference) (OtherBodyIndex :type Integer))
  ;[1 0 1] Jump up THROUGH Platform
  (if (== (Game|GetPlayerCharacter 0) OtherActor)
    (Collision|SetCollisionEnabled (Variables|Default|GetPlatform) "QueryAndPhysics")))

(event OnComponentBeginOverlap(TopCollision)
  (params (OverlappedComponent :type Primitive%20Component%20Object%20Reference) (OtherActor :type Actor%20Object%20Reference) (OtherComp :type Primitive%20Component%20Object%20Reference) (OtherBodyIndex :type Integer) (bFromSweep :type Boolean) (SweepResult :type Hit%20Result%20Structure%20%28by%20ref%29))
  ;[1 0 1] Set Boolean for Detecting if Player is on TOP of the Platform
  (if (== OtherActor (Game|GetPlayerCharacter 0))
    (Variables|Default|SetIsPlayerOnOfPlatformTop? true)))

(event OnComponentEndOverlap(TopCollision)
  (params (OverlappedComponent :type Primitive%20Component%20Object%20Reference) (OtherActor :type Actor%20Object%20Reference) (OtherComp :type Primitive%20Component%20Object%20Reference) (OtherBodyIndex :type Integer))
  ;[1 0 1] Set Boolean for Detecting if Player is on TOP of the Platform
  (if (== (Game|GetPlayerCharacter 0) OtherActor)
    (Variables|Default|SetIsPlayerOnOfPlatformTop? false)))

(event Input|EnhancedActionEvents|EnhancedInputActionIA_PlayerDown
  (params (ActionValue :type Boolean) (ElapsedSeconds :type Float%20%28double-precision%29) (TriggeredSeconds :type Float%20%28double-precision%29) (InputAction :type Input%20Action%20Object%20Reference :default "/Game/ThirdPerson/Input/Actions/IA_PlayerDown.IA_PlayerDown"))
  ;[1 0 1] Allow Player to Drop Down Through Platform
  (:Started
    (if (Variables|Default|GetIsPlayerOnOfPlatformTop?)
      (Collision|SetCollisionEnabled (Variables|Default|GetPlatform) "NoCollision"))))

(fn ConstructionScript)